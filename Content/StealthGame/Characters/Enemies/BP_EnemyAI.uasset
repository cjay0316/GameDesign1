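; Stealth-game enemy that patrols, investigates noises and chases the player, without a behavior tree.
; Tick uses CanMove, CanChase and PlayerVisible flags to start AIMoveTo patrols (random or cycling target points) or chases, varying walk speed.
; PawnSensing triggers noise investigation and sightings, while a looping timer drops stale sightings.
; Arrivals trigger a DoOnce-gated attack montage, whose notify sphere-traces from the hand and reloads a hit player's checkpoint.
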(event `self.PawnSensing.OnHearNoise`
  (params (Instigator :type "Pawn Object Reference") (Location :type "Vector Structure (by ref)") (Volume :type "Float (single-precision)"))
  (if (not (`self.bPlayerVisible`))
    (`KismetSystemLibrary.PrintString` "WHAT WAS THAT SOUND?")
    (`self.UpdateWalkSpeed` 275.0)
    (set `self.bCanMove` false)
    (`|AIMoveTo` self Location null
      (:`OnSuccess`
        (`KismetSystemLibrary.Delay` 0.5)
        (`KismetSystemLibrary.PrintString` "Gotcha!")
        (`self.Attack`)
        (`KismetSystemLibrary.Delay` 4.0)
        (`KismetSystemLibrary.PrintString` "You better run and hide!")
        (set `self.bCanMove` true)))))

(event `self.PawnSensing.OnSeePawn`
  (params (Pawn :type "Pawn Object Reference"))
  (if (`self.ActorHasTag` Pawn "Player")
    (`KismetSystemLibrary.PrintString` "I SEE YOU!")
    (set `self.bPlayerVisible` true)
    (set `self.LastSeenTime` (`GameplayStatics.GetTimeSeconds`))
    (bind _returnvalue (`KismetSystemLibrary.K2_SetTimer` null "CheckLastSight" 0.5 true))
    (set `self.SightHandle` _returnvalue)))

(event `ChasePlayer`
  (`self.UpdateWalkSpeed` 500.0)
  (set `self.bCanMove` false)
  (set `self.bCanChase` false)
  (`|AIMoveTo` self (0.0 0.0 0.0) (`GameplayStatics.GetPlayerPawn` 0)
    (:`OnSuccess`
      (`self.Attack`))
    (:`OnFail`
      _))
  (`KismetSystemLibrary.Delay` 2.0)
  (set `self.bCanMove` true)
  (set `self.bCanChase` true))

(event `Random Patrol`
  (`self.UpdateWalkSpeed` 300.0)
  (set `self.bCanMove` false)
  (`|AIMoveTo` self (`NavigationSystemV1.K2_GetRandomReachablePointInRadius` (`self.K2_GetActorLocation`) 2000.0 null null) null
    (:`OnSuccess`
      (`KismetSystemLibrary.Delay` 2.0)
      (set `self.bCanMove` true))))

(event `self.ReceiveTick`
  (params (DeltaSeconds :type "Float (single-precision)"))
  (if (`self.bCanMove`)
    (if (`self.bPlayerVisible`)
      (`self.ChasePlayer`)
      (else
        (switch `/Game/StealthGame/Characters/Enemies/EParolType` (`self.PatrolType`)
          (:`NewEnumerator0`
            (`self.PatrolTargets`))
          (:`NewEnumerator2`
            (`self.Random Patrol`)))))
    (elif (and (`self.bCanChase`) (`self.bPlayerVisible`))
      (`MovementComponent.StopMovementImmediately` (`self.CharacterMovement`))
      (`self.ChasePlayer`))))

(event `PatrolTargets`
  (`self.MoveToNextTargetPoint`))

(event `GetNextPatrolPoint`
  (set `self.CurrentIndex` (mod (+ (`self.CurrentIndex`) 1) (`KismetArrayLibrary.Array_Length` (`self.PatrolTargetPoints`)))))

(event `MoveToNextTargetPoint`
  (`self.UpdateWalkSpeed` 100.0)
  (set `self.bCanMove` false)
  (`|AIMoveTo` self (0.0 0.0 0.0) (`|GetArrayItem` (`self.PatrolTargetPoints`) (`self.CurrentIndex`))
    (:`OnSuccess`
      (`KismetSystemLibrary.PrintString` "You here?")
      (`KismetSystemLibrary.Delay` 0.2)
      (`self.Attack`)
      (`KismetSystemLibrary.Delay` 2.0)
      (`KismetSystemLibrary.PrintString` "Nope. I'll find you!")
      (`self.GetNextPatrolPoint`)
      (set `self.bCanMove` true))))

(event `CheckLastSight`
  (if (> (- (`GameplayStatics.GetTimeSeconds`) (`self.LastSeenTime`)) (`self.SightInterval`))
    (set `self.bPlayerVisible` false)
    (`KismetSystemLibrary.K2_ClearAndInvalidateTimerHandle` (`self.SightHandle`))
    (`KismetSystemLibrary.PrintString` "target lost")))

(event `Attack`
  (bind _returnvalue (`SceneComponent.GetSocketLocation` (`self.Mesh`) "hand_r"))
  ; Melee Attack
  (`/Engine/EditorBlueprintResources/StandardMacros.DoOnce` false :!label _label
    (:`Completed`
      (bind _notifyname (`|PlayMontage` (`self.Mesh`) "/Game/StealthGame/Characters/Enemies/AM_Attack_01.AM_Attack_01")
        (:`OnCompleted`
          (`self.ResetAttack`))
        (:`OnNotifyBegin`
          (switch `name` _notifyname
            (:`AttackDamage`
              (`KismetSystemLibrary.PrintString` "Im Attacking")
              (bind (_outhits _returnvalue_2) (`KismetSystemLibrary.SphereTraceMultiForObjects` :`Start` _returnvalue :`End` (+ _returnvalue (* (`self.GetActorForwardVector`) (`self.MeleeTraceDistance`))) :`Radius` (`self.MeleeTraceRadius`) :`ObjectTypes` (`|MakeArray` "ObjectTypeQuery3" :!type "EObjectTypeQuery Enum") :`DrawDebugType` "ForOneFrame"))
              (if _returnvalue_2
                (for _array_element _outhits
                  (bind _asbp_third_person_character_custom (cast `/Game/StealthGame/Core/Characters/PlayerCharacter/BP_ThirdPersonCharacterCustom` (`.HitActor` (`GameplayStatics.BreakHitResult` _array_element))))
                  (`/Game/StealthGame/Core/Characters/PlayerCharacter/BP_ThirdPersonCharacterCustom.Load Checkpoint` _asbp_third_person_character_custom))))))))))

(event `ResetAttack`
  ; Melee Attack
  (goto _label :!via `Reset`))

(fn `UpdateWalkSpeed`
  (params (NewWalkingSpeed :type "Float (double-precision)"))
  (set `CharacterMovementComponent.MaxWalkSpeed` NewWalkingSpeed (`self.CharacterMovement`)))

(fn `UserConstructionScript`)